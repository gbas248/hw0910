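; Monster enemy that wanders randomly, chases and attacks the player, and takes bullet damage.
; A self-repeating AIMoveTo loop picks roaming or chasing from a seen flag set by pawn sensing or non-lethal hits, and cleared when the chase fails.
; Attacks halt movement and briefly enable overlap events on an attack area that damages the player.
; Lethal bullets trigger ragdoll, increment the game mode's kill count and destroy the monster after a delay.
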(event OnSeePawn(感測元件)
  (params (Pawn :type Pawn%20Object%20Reference))
  (bind _charactermovement (Variables|Character|GetCharacterMovement))
  ;[1 1 1] 看到玩家後保存資訊
  (bind _asbp玩家 (Utilities|Casting|CastToBP玩家 Pawn))
  (Variables|Default|Set玩家控制 _asbp玩家)
  (Variables|Default|Set是否看到玩家 true)
  (Variables|Default|Set停留的最大值 0.0)
  (Utilities|FlowControl|DoOnce false
    (:Completed
      ;[1 1 1] 判斷有沒有看到玩家
      (if (Variables|Default|Get是否看到玩家) :!label _label
        ;[1 1 1] 看到玩家
        (AI|AIMoveTo self "0, 0, 0" (Variables|Default|Get玩家控制) (Variables|Default|Get停止半徑) false
          (:OnSuccess
            ;[1 1 1] 攻擊狀態
            (Variables|Default|Set攻擊中 true)
            (Variables|/Script/Engine.CharacterMovementComponent|SetMaxWalkSpeed _charactermovement 0.0)
            (Utilities|FlowControl|Delay 1.0)
            (Variables|/Script/Engine.PrimitiveComponent|SetbGenerateOverlapEvents (Variables|Default|Get攻擊區域) true) ; 開啟碰撞
            (Utilities|FlowControl|Delay 0.3)
            (Variables|/Script/Engine.PrimitiveComponent|SetbGenerateOverlapEvents (Variables|Default|Get攻擊區域) false) ; 關閉碰撞
            (Utilities|FlowControl|Delay 1.0)
            (Variables|/Script/Engine.CharacterMovementComponent|SetMaxWalkSpeed _charactermovement 5e+02)
            (Variables|Default|Set攻擊中 false)
            (goto _label))
          (:OnFail
            (Variables|Default|Set是否看到玩家 false)
            (Variables|Default|Set停留的最大值 3.0)
            (goto _label)))
        (else
          ;[1 0.6201 0.4062] 沒看到玩家隨機走動
          (AI|AIMoveTo self (.RandomLocation (AI|Navigation|GetRandomReachablePointinRadius (Transformation|GetWorldLocation (Variables|Collision|GetCapsuleComponent)) (Variables|Default|Get隨機走動半徑) 0 0)) 0 (Variables|Default|Get停止半徑) false ; ai移動到的地方
            (:then
              ;[1 0.5748 0.9932] 隨機停留
              (Utilities|FlowControl|Delay (* (Math|Random|RandomFloat) (Variables|Default|Get停留的最大值)))
              (goto _label))))))))

(event OnComponentBeginOverlap(CapsuleComponent)
  (params (OverlappedComponent :type Primitive%20Component%20Object%20Reference) (OtherActor :type Actor%20Object%20Reference) (OtherComp :type Primitive%20Component%20Object%20Reference) (OtherBodyIndex :type Integer) (bFromSweep :type Boolean) (SweepResult :type Hit%20Result%20Structure%20%28by%20ref%29))
  (bind _charactermovement (Variables|Character|GetCharacterMovement))
  (bind _遊戲模式 (Variables|Default|Get遊戲模式))
  ;[1 1 1] 受傷和死亡
  (bind _asbp_子彈 (Utilities|Casting|CastToBP_子彈 OtherActor))
  (bind _是否死亡 (CallFunction|受傷 (Variables|/Game/BP/BP_子彈.BP_子彈_C|Get目前武器傷害 _asbp_子彈)))
  (if _是否死亡
    (Variables|/Game/BP/BP遊戲.BP遊戲_C|Set擊殺怪物數量 _遊戲模式 (+ (Variables|/Game/BP/BP遊戲.BP遊戲_C|Get擊殺怪物數量 _遊戲模式) 1))
    (Utilities|FlowControl|Delay 5.0)
    (Actor|DestroyActor)
    (else
      ;[1 1 1] 看到玩家後保存資訊
      (Variables|Default|Set是否看到玩家 true)
      (Variables|Default|Set停留的最大值 0.0)
      (Utilities|FlowControl|DoOnce false
        (:Completed
          ;[1 1 1] 判斷有沒有看到玩家
          (if (Variables|Default|Get是否看到玩家) :!label _label
            ;[1 1 1] 看到玩家
            (AI|AIMoveTo self "0, 0, 0" (Variables|Default|Get玩家控制) (Variables|Default|Get停止半徑) false
              (:OnSuccess
                ;[1 1 1] 攻擊狀態
                (Variables|Default|Set攻擊中 true)
                (Variables|/Script/Engine.CharacterMovementComponent|SetMaxWalkSpeed _charactermovement 0.0)
                (Utilities|FlowControl|Delay 1.0)
                (Variables|/Script/Engine.PrimitiveComponent|SetbGenerateOverlapEvents (Variables|Default|Get攻擊區域) true) ; 開啟碰撞
                (Utilities|FlowControl|Delay 0.3)
                (Variables|/Script/Engine.PrimitiveComponent|SetbGenerateOverlapEvents (Variables|Default|Get攻擊區域) false) ; 關閉碰撞
                (Utilities|FlowControl|Delay 1.0)
                (Variables|/Script/Engine.CharacterMovementComponent|SetMaxWalkSpeed _charactermovement 5e+02)
                (Variables|Default|Set攻擊中 false)
                (goto _label))
              (:OnFail
                (Variables|Default|Set是否看到玩家 false)
                (Variables|Default|Set停留的最大值 3.0)
                (goto _label)))
            (else
              ;[1 0.6201 0.4062] 沒看到玩家隨機走動
              (AI|AIMoveTo self (.RandomLocation (AI|Navigation|GetRandomReachablePointinRadius (Transformation|GetWorldLocation (Variables|Collision|GetCapsuleComponent)) (Variables|Default|Get隨機走動半徑) 0 0)) 0 (Variables|Default|Get停止半徑) false ; ai移動到的地方
                (:then
                  ;[1 0.5748 0.9932] 隨機停留
                  (Utilities|FlowControl|Delay (* (Math|Random|RandomFloat) (Variables|Default|Get停留的最大值)))
                  (goto _label))))))))))

(event OnComponentBeginOverlap(攻擊區域)
  (params (OverlappedComponent :type Primitive%20Component%20Object%20Reference) (OtherActor :type Actor%20Object%20Reference) (OtherComp :type Primitive%20Component%20Object%20Reference) (OtherBodyIndex :type Integer) (bFromSweep :type Boolean) (SweepResult :type Hit%20Result%20Structure%20%28by%20ref%29))
  ;[1 1 1] 攻擊區域及傳送傷害
  (bind _asbp玩家 (Utilities|Casting|CastToBP玩家 OtherActor))
  (Default|受傷 _asbp玩家 (Variables|Default|Get攻擊力)))

(event EventBeginPlay
  (bind _charactermovement (Variables|Character|GetCharacterMovement))
  (Utilities|FlowControl|Sequence
    (:then_0
      ;[1 1 1] 判斷有沒有看到玩家
      (if (Variables|Default|Get是否看到玩家) :!label _label
        ;[1 1 1] 看到玩家
        (AI|AIMoveTo self "0, 0, 0" (Variables|Default|Get玩家控制) (Variables|Default|Get停止半徑) false
          (:OnSuccess
            ;[1 1 1] 攻擊狀態
            (Variables|Default|Set攻擊中 true)
            (Variables|/Script/Engine.CharacterMovementComponent|SetMaxWalkSpeed _charactermovement 0.0)
            (Utilities|FlowControl|Delay 1.0)
            (Variables|/Script/Engine.PrimitiveComponent|SetbGenerateOverlapEvents (Variables|Default|Get攻擊區域) true) ; 開啟碰撞
            (Utilities|FlowControl|Delay 0.3)
            (Variables|/Script/Engine.PrimitiveComponent|SetbGenerateOverlapEvents (Variables|Default|Get攻擊區域) false) ; 關閉碰撞
            (Utilities|FlowControl|Delay 1.0)
            (Variables|/Script/Engine.CharacterMovementComponent|SetMaxWalkSpeed _charactermovement 5e+02)
            (Variables|Default|Set攻擊中 false)
            (goto _label))
          (:OnFail
            (Variables|Default|Set是否看到玩家 false)
            (Variables|Default|Set停留的最大值 3.0)
            (goto _label)))
        (else
          ;[1 0.6201 0.4062] 沒看到玩家隨機走動
          (AI|AIMoveTo self (.RandomLocation (AI|Navigation|GetRandomReachablePointinRadius (Transformation|GetWorldLocation (Variables|Collision|GetCapsuleComponent)) (Variables|Default|Get隨機走動半徑) 0 0)) 0 (Variables|Default|Get停止半徑) false ; ai移動到的地方
            (:then
              ;[1 0.5748 0.9932] 隨機停留
              (Utilities|FlowControl|Delay (* (Math|Random|RandomFloat) (Variables|Default|Get停留的最大值)))
              (goto _label))))))
    (:then_1
      ;[0.3801 0.7434 1] 取得遊戲模式
      (bind _asbp遊戲 (Utilities|Casting|CastToBP遊戲 (Game|GetGameMode)))
      (Variables|Default|Set遊戲模式 _asbp遊戲))))

(fn ConstructionScript)

(fn 受傷
  (params (接收到傷害 :type Float%20%28single-precision%29))
  ;[1 1 1] 受傷
  (bind _output_get (Variables|Default|Set血量 (- (Variables|Default|Get血量) 接收到傷害)))
  (if (<= _output_get 0.0)
    ;[1 1 1] 死亡
    (Physics|SetSimulatePhysics (Variables|Character|GetMesh) true) ; 模擬布偶效果
    (Collision|SetCollisionEnabled (Variables|Collision|GetCapsuleComponent) "NoCollision") ; 設定碰撞啟動:現在為關閉膠囊碰撞
    (return true)
    (else
      (return false))))